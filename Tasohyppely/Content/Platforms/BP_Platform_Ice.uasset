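; Ice platform that changes how characters move while they are on it by altering their ground friction, acceleration and walking braking.
; Activate Platform writes the platform's movement values to the indexed overlapping character's movement component.
; Deactivate Platform removes the character from the list and restores hardcoded movement values, skipping the reset when an overlap check filtered to ice platforms passes.
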(event EventBeginPlay
  (|CallParentFunction) ; This node is disabled and will not be called.\nDrag off pins to build functionality.
)

(event Collision|EventActorBeginOverlap
  (params (OtherActor :type Actor%20Object%20Reference))
  (|CallParentFunction OtherActor) ; This node is disabled and will not be called.\nDrag off pins to build functionality.
)

(event EventTick
  (params (DeltaSeconds :type Float%20%28single-precision%29)))

(fn ConstructionScript
  (|CallParentFunction))

(fn ActivatePlatform
  (params (Index :type Integer))
  (bind _overlapping_actors (Variables|Default|GetOverlapping%20Actors))
  (bind _output (Utilities|Array|Get(acopy) _overlapping_actors Index))
  (bind _charactermovement (Variables|/Script/Engine.Character|GetCharacterMovement _output))
  (Variables|/Script/Engine.CharacterMovementComponent|SetGroundFriction _charactermovement (Variables|Default|GetGround%20Friction))
  (Variables|/Script/Engine.CharacterMovementComponent|SetMaxAcceleration _charactermovement (Variables|Default|GetMax%20Acceleration))
  (Variables|/Script/Engine.CharacterMovementComponent|SetBrakingDecelerationWalking _charactermovement (Variables|Default|GetBraking%20Deceleration%20Walking)))

(fn DeactivatePlatform
  (params (Index :type Integer))
  (bind _output_get (LocalVariables|SetCharacter (Utilities|Array|Get(acopy) (Variables|Default|GetOverlapping%20Actors) Index)))
  (if (CallFunction|CheckOverlapActor _output_get "BP_Platform_Ice_C")
    (Utilities|Array|RemoveIndex (Variables|Default|GetOverlapping%20Actors) Index)
    (else
      (Variables|/Script/Engine.CharacterMovementComponent|SetGroundFriction (Variables|/Script/Engine.Character|GetCharacterMovement (LocalVariables|GetCharacter)) 8.0)
      (Variables|/Script/Engine.CharacterMovementComponent|SetMaxAcceleration (Variables|/Script/Engine.Character|GetCharacterMovement (LocalVariables|GetCharacter)) 1.5e+03)
      (Variables|/Script/Engine.CharacterMovementComponent|SetBrakingDecelerationWalking (Variables|/Script/Engine.Character|GetCharacterMovement (LocalVariables|GetCharacter)) 2e+03)
      (Utilities|Array|RemoveIndex (Variables|Default|GetOverlapping%20Actors) Index))))