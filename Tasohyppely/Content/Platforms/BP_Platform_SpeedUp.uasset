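; Speed boost platform Blueprint that changes a Character's walk speed by AddSpeed, building on CheckOverlapping and OverlappingActors, which are defined outside this file.
; ActivatePlatform adds AddSpeed to MaxWalkSpeed, though nothing here calls it.
; On end overlap, a tracked Character waits SpeedDuration before DeactivatePlatform removes it from the array.
; Deactivation sets speed to AddSpeed minus current speed, so it does not restore the original.
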(event EventBeginPlay
  (|CallParentFunction) ; This node is disabled and will not be called.\nDrag off pins to build functionality.
)

(event Collision|EventActorBeginOverlap
  (params (OtherActor :type Actor%20Object%20Reference))
  (|CallParentFunction OtherActor) ; This node is disabled and will not be called.\nDrag off pins to build functionality.
)

(event EventActorEndOverlap
  (params (OtherActor :type Actor%20Object%20Reference))
  (bind _ascharacter (Utilities|Casting|CastToCharacter OtherActor))
  (if (.IsOverlapping? (CallFunction|CheckOverlapping _ascharacter))
    (Utilities|FlowControl|Delay (Variables|Default|GetSpeed%20Duration))
    (CallFunction|DeactivatePlatform (.Index (CallFunction|CheckOverlapping _ascharacter)))))

(fn ConstructionScript
  (|CallParentFunction))

(fn ActivatePlatform
  (params (Index :type Integer))
  (bind _overlapping_actors (Variables|Default|GetOverlapping%20Actors))
  (bind _output (Utilities|Array|Get(acopy) _overlapping_actors Index))
  (bind _charactermovement (Variables|/Script/Engine.Character|GetCharacterMovement _output))
  (Variables|/Script/Engine.CharacterMovementComponent|SetMaxWalkSpeed _charactermovement (+ (Variables|/Script/Engine.CharacterMovementComponent|GetMaxWalkSpeed _charactermovement) (Variables|Default|GetAdd%20Speed)))
  (Development|PrintString "Activate"))

(fn DeactivatePlatform
  (params (Index :type Integer))
  (bind _overlapping_actors (Variables|Default|GetOverlapping%20Actors))
  (bind _output (Utilities|Array|Get(acopy) _overlapping_actors Index))
  (bind _charactermovement (Variables|/Script/Engine.Character|GetCharacterMovement _output))
  (Variables|/Script/Engine.CharacterMovementComponent|SetMaxWalkSpeed _charactermovement (- (Variables|Default|GetAdd%20Speed) (Variables|/Script/Engine.CharacterMovementComponent|GetMaxWalkSpeed _charactermovement)))
  (Development|PrintString "Deactivate")
  (Utilities|Array|RemoveIndex (Variables|Default|GetOverlapping%20Actors) Index))