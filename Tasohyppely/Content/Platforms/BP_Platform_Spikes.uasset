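; BP_Platform_Spikes is a spike platform that kills the player character.
; Its Activate Platform function takes an index into OverlappingActors, casts that actor to BP_ThirdPersonCharacter and calls KillPlayer on it.
; It then removes that entry from the array if the actor is still valid.
; The event graph holds only disabled stubs, so this file does not show what fills the array or triggers activation.
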(event EventBeginPlay
  (|CallParentFunction) ; This node is disabled and will not be called.\nDrag off pins to build functionality.
)

(event Collision|EventActorBeginOverlap
  (params (OtherActor :type Actor%20Object%20Reference))
  (|CallParentFunction OtherActor) ; This node is disabled and will not be called.\nDrag off pins to build functionality.
)

(fn ConstructionScript
  (|CallParentFunction))

(fn ActivatePlatform
  (params (Index :type Integer))
  (bind _asbp_third_person_character (Utilities|Casting|CastToBP_ThirdPersonCharacter (Utilities|Array|Get(acopy) (Variables|Default|GetOverlapping%20Actors) Index)))
  (Default|KillPlayer _asbp_third_person_character)
  (Utilities|IsValid (Utilities|Array|Get(acopy) (Variables|Default|GetOverlapping%20Actors) Index)
    (:Is%20Valid
      (Utilities|Array|RemoveIndex (Variables|Default|GetOverlapping%20Actors) Index))))